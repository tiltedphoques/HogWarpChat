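; BP_HogWarpChat is an actor that manages the on-screen chat widget, creating it hidden at BeginPlay and focusing it on Enter.
; RecieveMsg adds a message, shows the widget, plays a sound, then triggers a retriggerable delay before a timeline fades it out unless focused.
; Tick currently spams a delayed test message to check text wrapping.
; SendMsg and RecieveMsgs are empty stubs.
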(event `self.ReceiveTick`
  (params (DeltaSeconds :type "Float (single-precision)"))
  (`KismetSystemLibrary.Delay` 1.0)
  (`self.RecieveMsg` "Jay-Jay: Hey How you doing this is a very long message just to test text wrap, but i'll also spam it so that we are getting a fair chunk of messages coming throuhg to see how it handles this kind of hting."))

(event `self.ReceiveBeginPlay`
  (bind _returnvalue (`GameplayStatics.GetPlayerController` 0))
  (`self.EnableInput` _returnvalue)
  (bind _returnvalue_2 (`|CreateWidget` "/HogWarpChat/Widgets/W_HogWarpChat.W_HogWarpChat_C" _returnvalue self))
  (bind _output_get (set `self.UI_Chat` _returnvalue_2))
  (`UserWidget.AddToViewport` _output_get 0)
  (`Widget.SetVisibility` _output_get "Hidden")
  (add `self.MessageSend` (`|CreateDelegate` :!event `SendMsg`)))

(event `Key|Enter` :consume false :overrideparent false
  (params (Key :type "Key Structure"))
  (bind _ui_chat (`self.UI_Chat`))
  (:`Pressed`
    (`/HogWarpChat/Widgets/W_HogWarpChat.SetFocused` _ui_chat true)
    (`/HogWarpChat/Widgets/W_HogWarpChat.SetView` _ui_chat true)))

(event `self.ReceiveDestroyed`
  (bind _ui_chat (`self.UI_Chat`))
  (`/Engine/EditorBlueprintResources/StandardMacros.IsValid` _ui_chat
    (:`Is Valid`
      (`Widget.RemoveFromParent` _ui_chat))))

(event `StartFade`
  (bind _ui_chat (`self.UI_Chat`))
  (`KismetSystemLibrary.RetriggerableDelay` (`self.StartFadeDelay`))
  (if (not (`/HogWarpChat/Widgets/W_HogWarpChat.Focused` (`self.UI_Chat`)))
    (bind (_direction _fade) (`Timeline|FadeChat` :!via `PlayFromStart` :!label _label)
      (:`Update`
        (if (`/HogWarpChat/Widgets/W_HogWarpChat.Focused` (`self.UI_Chat`))
          (`self.SetVisible`)
          (goto _label :!via `Stop`)
          (else
            (`Widget.SetRenderOpacity` _ui_chat _fade))))
      (:`Finished`
        (`Widget.SetVisibility` _ui_chat "Hidden")))))

(fn `RecieveMsg`
  (params (Message :type String))
  (bind _ui_chat (`self.UI_Chat`))
  (`/HogWarpChat/Widgets/W_HogWarpChat.AddMessage` (`self.UI_Chat`) Message)
  (`self.SetVisible`)
  (`self.StartFade`)
  (`AkGameplayStatics.PostEventAtLocation` "/Game/WWise/Events/UI/Menu/UI_Menu_Select.UI_Menu_Select") ; SFX
  (if (not (`Widget.HasKeyboardFocus` (`/HogWarpChat/Widgets/W_HogWarpChat.inputText` _ui_chat)))
    (`/HogWarpChat/Widgets/W_HogWarpChat.SetView` _ui_chat false)))

(fn `RecieveMsgs`)

(fn `SendMsg`
  (params (Message :type String)))

(fn `SetVisible`
  (bind _ui_chat (`self.UI_Chat`))
  (`Widget.SetVisibility` _ui_chat "Visible")
  (`Widget.SetRenderOpacity` _ui_chat 1.0))

(fn `UserConstructionScript`)